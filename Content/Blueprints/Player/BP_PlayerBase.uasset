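; Base player character Blueprint for a wave-based shooter, handling rifle fire, reloading, health and death.
; FiringWeapon spends ammo and line-traces from BulletSpawner, damaging actors tagged Enemy, with muzzle flash and sounds.
; Reload plays a montage, refills ammo immediately and blocks firing through a delay.
; Ammo and health update the PlayerController's HUD; death disables collision and movement, then shows game over with the GameMode's wave.
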(event `self.ReceiveBeginPlay`
  (bind _playercontroller (message `/Game/Blueprints/Interfaces/INT_PlayerController.GetPlayerControllerRef` (`GameplayStatics.GetPlayerController` 0)))
  (set `self.Player Controller` _playercontroller)
  (bind _gamemode (message `/Game/Blueprints/Interfaces/INT_GameMode.GetGameModeRef` (`GameplayStatics.GetGameMode`)))
  (set `self.Game Mode` _gamemode)
  (`/Game/UI/WB_Main.SetAmmo` (`/Game/Blueprints/PC_ShooterGameProject.WB_Main` (`self.Player Controller`)) (`self.CurrentAmmo`) (`self.MaxAmmo`)))

(event `/Game/Blueprints/Interfaces/INT_PlayerBase.FiringWeapon`
  (bind (_location _rotation) (`self.GetBulletLocAndRot`))
  (bind (_location_2 _rotation_2) (`self.GetBulletLocAndRot`))
  (bind _maxammo (`self.MaxAmmo`))
  (if (and (not (`self.bIsDead`)) (not (`self.bIsReloading`)))
    (bind _result (`/Engine/EditorBlueprintResources/StandardMacros.DecrementInt` (`self.CurrentAmmo`))
      (:`  `
        (bind _returnvalue (`KismetMathLibrary.Clamp` _result 0 _maxammo))
        (`/Game/UI/WB_Main.SetAmmo` (`/Game/Blueprints/PC_ShooterGameProject.WB_Main` (`self.Player Controller`)) _returnvalue _maxammo)
        (if (> _returnvalue 0)
          (`GameplayStatics.PlaySoundAtLocation` "/Game/MilitaryWeapDark/Sound/Rifle/RifleB_Fire_Cue.RifleB_Fire_Cue" (`self.K2_GetActorLocation`) (struct) 1.0 1.0 0.0 null null null null)
          (`GameplayStatics.SpawnEmitterAttached` "/Game/MilitaryWeapDark/FX/P_AssaultRifle_MuzzleFlash.P_AssaultRifle_MuzzleFlash" (`self.BulletSpawner`) "None" _location_2 _rotation_2 (1.0 1.0 1.0) "KeepWorldPosition")
          (bind _outhit (`KismetSystemLibrary.LineTraceSingle` _location (+ _location (* (`KismetMathLibrary.GetForwardVector` _rotation) (`self.FirringDistance`))) "TraceTypeQuery1"))
          (bind (_bblockinghit _binitialoverlap _time _distance _location_3 _impactpoint _normal _impactnormal _physmat _hitactor) (`GameplayStatics.BreakHitResult` _outhit))
          (if (`self.ActorHasTag` _hitactor "Enemy")
            (`GameplayStatics.ApplyDamage` _hitactor 25.0 (`GameplayStatics.GetPlayerController` 0) self)
            (`GameplayStatics.PlaySoundAtLocation` "/Game/MilitaryWeapDark/Sound/Rifle/Rifle_ImpactBody_Cue.Rifle_ImpactBody_Cue" _location_3 (struct) 1.0 1.0 0.0 null null null null)))))))

(event `InputAction|Reload`
  (params (Key :type "Key Structure"))
  (:`Pressed`
    (if (and (not (`self.bIsDead`)) (not (`self.bIsReloading`)) (!= (`self.CurrentAmmo`) (`self.MaxAmmo`)))
      (set `self.bIsReloading` true)
      (`|PlayMontage` (`self.Mesh`) "/Game/Assets/Characters/Animations/AnimMon_Reload.AnimMon_Reload"
        (:`then`
          (bind _output_get (set `self.CurrentAmmo` 30))
          (`/Game/UI/WB_Main.SetAmmo` (`/Game/Blueprints/PC_ShooterGameProject.WB_Main` (`self.Player Controller`)) _output_get (`self.MaxAmmo`))
          (`KismetSystemLibrary.Delay` 2.0)
          (set `self.bIsReloading` false))))))

(event `self.ReceiveAnyDamage`
  (params (Damage :type "Float (single-precision)") (DamageType :type "DamageType Object Reference") (InstigatedBy :type "Controller Object Reference") (DamageCauser :type "Actor Object Reference"))
  (bind _output_get (set `self.Health` (`KismetMathLibrary.FClamp` (- (`self.Health`) Damage) 0.0 100.0)))
  (`/Game/UI/WB_Main.SetPlayerHealth` (`/Game/Blueprints/PC_ShooterGameProject.WB_Main` (`self.Player Controller`)) _output_get)
  (if (== _output_get 0.0)
    (`/Game/Blueprints/Interfaces/INT_PlayerBase.PlayerDeath`)))

(event `/Game/Blueprints/Interfaces/INT_PlayerBase.PlayerDeath`
  (bind _player_controller (`self.Player Controller`))
  (bind _mesh (`self.Mesh`))
  (bind _wb_gameover (`/Game/Blueprints/PC_ShooterGameProject.WB_GameOver` _player_controller))
  (set `self.bIsDead` true)
  (`SkeletalMeshComponent.PlayAnimation` _mesh "/Game/Assets/Characters/Animations/Death_3.Death_3" false)
  (`PrimitiveComponent.SetCollisionEnabled` _mesh "NoCollision")
  (`PrimitiveComponent.SetCollisionEnabled` (`self.CapsuleComponent`) "NoCollision")
  (`CharacterMovementComponent.DisableMovement` (`self.CharacterMovement`))
  (`GameplayStatics.PlaySound2D` "/Game/Audio/SC_DeathPlayer.SC_DeathPlayer" 1.0 1.0 0.0 null null)
  (`KismetSystemLibrary.Delay` 3.0)
  (`/Game/UI/WB_GameOver.GameOverWave` _wb_gameover (`KismetTextLibrary.Conv_IntToText` (- (`/Game/Blueprints/GM_ShooterGameProject.Wave` (`self.Game Mode`)) 0)))
  (`Widget.RemoveFromParent` (`/Game/Blueprints/PC_ShooterGameProject.WB_Main` _player_controller))
  (`UserWidget.AddToViewport` _wb_gameover 0)
  (set `PlayerController.bShowMouseCursor` true (`self.Player Controller`)))

(fn `GetBulletLocAndRot`
  (returns (Location :type "Vector Structure") (Rotation :type "Rotator Structure"))
  (bind _bulletspawner (`self.BulletSpawner`))
  (return (`SceneComponent.K2_GetComponentLocation` _bulletspawner) (`SceneComponent.K2_GetComponentRotation` _bulletspawner)))

(fn `GetPlayerRef`
  (returns (Player :type "/Game/Blueprints/Player/BP_PlayerBase Object Reference"))
  (return self))

(fn `UserConstructionScript`
  (`parent.UserConstructionScript`))