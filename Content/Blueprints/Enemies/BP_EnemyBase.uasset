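; Base melee enemy that chases the player, attacks, and dies when its health runs out.
; AIMoveTo success starts an attack montage if the player lives; completion resumes the chase, though ChasePlayer's first call is external.
; The montage notify runs a sphere overlap for pawns, then damages the target with sound and particles.
; Death disables collision and movement, updates the game mode's enemy list and HUD count, and requests a spawn when none remain.
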(event `self.ReceiveBeginPlay`
  (bind _gamemode (message `/Game/Blueprints/Interfaces/INT_GameMode.GetGameModeRef` (`GameplayStatics.GetGameMode`)))
  (set `self.GameMode` _gamemode)
  (bind _playercontroller (message `/Game/Blueprints/Interfaces/INT_PlayerController.GetPlayerControllerRef` (`GameplayStatics.GetPlayerController` 0)))
  (set `self.Player Controller` _playercontroller)
  (`KismetSystemLibrary.Delay` 1.3))

(event `self.ReceiveAnyDamage`
  (params (Damage :type "Float (single-precision)") (DamageType :type "DamageType Object Reference") (InstigatedBy :type "Controller Object Reference") (DamageCauser :type "Actor Object Reference"))
  (bind _output_get (set `self.Health` (- (`self.Health`) Damage)))
  (if (<= _output_get 0.0)
    (`/Game/Blueprints/Interfaces/INT_EnemyBase.Death`)))

(event `/Game/Blueprints/Interfaces/INT_EnemyBase.Death`
  (bind _mesh (`self.Mesh`))
  (set `self.bIsDead` true)
  (`SkeletalMeshComponent.PlayAnimation` _mesh "/Game/Marketplace/UndeadPack/Zombie/Animations/Anim_Death.Anim_Death" false)
  (`PrimitiveComponent.SetCollisionEnabled` _mesh "NoCollision")
  (`PrimitiveComponent.SetCollisionEnabled` (`self.CapsuleComponent`) "NoCollision")
  (`CharacterMovementComponent.DisableMovement` (`self.CharacterMovement`))
  (`/Game/Blueprints/Interfaces/INT_EnemyBase.RemovePawn`)
  (`KismetSystemLibrary.Delay` 5.0)
  (`SceneComponent.SetVisibility` (`self.Mesh`) false false))

(event `/Game/Blueprints/Interfaces/INT_EnemyBase.RemovePawn`
  (bind _enemypawns (`/Game/Blueprints/GM_ShooterGameProject.EnemyPawns` (`self.GameMode`)))
  (bind _returnvalue (`KismetArrayLibrary.Array_Length` _enemypawns))
  (`KismetArrayLibrary.Array_RemoveItem` _enemypawns self)
  (`/Game/UI/WB_Main.SetEnemyAmount` (`/Game/Blueprints/PC_ShooterGameProject.WB_Main` (`self.Player Controller`)) (`KismetTextLibrary.Conv_IntToText` _returnvalue))
  (if (== _returnvalue 0)
    (message `/Game/Blueprints/Interfaces/INT_GameMode.SpawnEnemy` (`self.GameMode`))))

(event `/Game/Blueprints/Interfaces/INT_EnemyBase.ChasePlayer`
  (params (Target :type "Pawn Object Reference"))
  (`|AIMoveTo` self (0.0 0.0 0.0) Target
    (:`OnSuccess`
      (bind _player (message `/Game/Blueprints/Interfaces/INT_PlayerBase.GetPlayerRef` (`GameplayStatics.GetPlayerCharacter` 0)))
      (if (not (`/Game/Blueprints/Player/BP_PlayerBase.bIsDead` _player))
        (`/Game/Blueprints/Interfaces/INT_EnemyBase.AttackPlayer` Target)))))

(event `/Game/Blueprints/Interfaces/INT_EnemyBase.AttackPlayer`
  (params (Target :type "Pawn Object Reference"))
  (bind _returnvalue (`SceneComponent.K2_GetComponentLocation` (`self.Sphere`)))
  (if (not (`self.bIsDead`))
    (`|PlayMontage` (`self.Mesh`) (`self.AttackAnim`)
      (:`OnCompleted`
        (`/Game/Blueprints/Interfaces/INT_EnemyBase.ChasePlayer` Target))
      (:`OnNotifyBegin`
        (`GameplayStatics.PlaySoundAtLocation` "/Game/MilitaryWeapDark/Sound/Knife/Knife_ImpactBody_Cue.Knife_ImpactBody_Cue" _returnvalue (struct) 1.0 1.0 0.0 null null null null)
        (bind (_outactors _returnvalue_2) (`KismetSystemLibrary.SphereOverlapActors` _returnvalue 100.0 (`|MakeArray` "ObjectTypeQuery3" :!type "EObjectTypeQuery Enum")))
        (if _returnvalue_2
          (`GameplayStatics.ApplyDamage` Target (`self.Damage`))
          (`GameplayStatics.PlaySoundAtLocation` "/Game/Marketplace/Sounds/male_hurt.male_hurt" _returnvalue (struct) 1.0 1.0 0.0 null null null null)
          (bind _player (message `/Game/Blueprints/Interfaces/INT_PlayerBase.GetPlayerRef` (`GameplayStatics.GetPlayerCharacter` 0)))
          (`GameplayStatics.SpawnEmitterAtLocation` "/Game/MilitaryWeapDark/FX/P_Grenade_MuzzleFlash_01.P_Grenade_MuzzleFlash_01" (`self.K2_GetActorLocation` _player) (struct) (2.0 2.0 2.0)))))))

(fn `GetEnemyRef`
  (returns (Enemy :type "/Game/Blueprints/Enemies/BP_EnemyBase Object Reference"))
  (return self))

(fn `UserConstructionScript`
  (`parent.UserConstructionScript`))